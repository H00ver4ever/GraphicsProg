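; BP_Char is the first-person shooter player character, providing basic movement, look and jump controls.
; Vertical and Horizontal axis inputs move it along the actor's forward and right vectors, while LookVertical and LookHorizontal feed controller pitch and yaw.
; The Jump action calls Jump on press, BeginPlay prints a spawn debug message, and the construction script is empty.
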(event `self.ReceiveBeginPlay`
  (`KismetSystemLibrary.PrintString` "Spawning Player " true true (struct :`G` 0.66 :`B` 1.0 :`A` 1.0) 5.0))

(event `InputAxis|Vertical`
  (params (AxisValue :type "Float (single-precision)"))
  (`self.AddMovementInput` (`self.GetActorForwardVector`) AxisValue))

(event `InputAxis|LookVertical`
  (params (AxisValue :type "Float (single-precision)"))
  (`self.AddControllerPitchInput` AxisValue))

(event `InputAxis|Horizontal`
  (params (AxisValue :type "Float (single-precision)"))
  (`self.AddMovementInput` (`self.GetActorRightVector`) AxisValue))

(event `InputAxis|LookHorizontal`
  (params (AxisValue :type "Float (single-precision)"))
  (`self.AddControllerYawInput` AxisValue))

(event `InputAction|Jump`
  (params (Key :type "Key Structure"))
  (:`Pressed`
    (`self.Jump`)))

(fn `UserConstructionScript`)